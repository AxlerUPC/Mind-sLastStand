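; Health component that offers functions for healing and damage, reporting each result through debug print strings.
; Curarse adds health to SaludActual, clamped between zero and SaludMaxima.
; RealizarDaño zeroes SaludActual, then clamps the damage to choose a destroyed or damaged message.
; DañoARecibir writes damage minus current health into SaludMaxima, leaves SaludActual unchanged, and prints death when SaludActual is above zero.
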(event EventBeginPlay)

(event EventTick
  (params (DeltaSeconds :type Float%20%28single-precision%29)))

(fn Curarse
  (params (Salud%20a%20añadir :type Float%20%28double-precision%29))
  (bind _output_get (Variables|Default|SetSaludActual (Math|Float|Clamp(Float) (+ (Variables|Default|GetSaludActual) Salud%20a%20añadir) 0.0 (Variables|Default|GetSaludMaxima))))
  (Development|PrintString (Utilities|String|Append "Te curaste:" (Utilities|String|ToString(Float) _output_get))))

(fn RealizarDaño
  (params (Daño :type Float%20%28double-precision%29))
  (bind _output_get (Variables|Default|SetSaludActual 0.0))
  (if (== (Math|Float|Clamp(Float) (- Daño (Variables|Default|GetSaludActual)) 0.0 (Variables|Default|GetSaludMaxima)) 0.0)
    (Development|PrintString "Objeto o enemigo Destruido")
    (else
      (Development|PrintString (Utilities|String|Append "Recibio daño" (Utilities|String|ToString(Float) _output_get))))))

(fn DañoARecibir
  (params (DañoRecibido :type Float%20%28double-precision%29))
  (bind _output_get (Variables|Default|SetSaludMaxima (- DañoRecibido (Variables|Default|GetSaludActual))))
  (if (> (Variables|Default|GetSaludActual) 0.0)
    (Development|PrintString "Moriste")
    (else
      (Development|PrintString (Utilities|String|Append "Recibiste Daño" (Utilities|String|ToString(Float) DañoRecibido) "Vida Restante" (Utilities|String|ToString(Float) _output_get))))))